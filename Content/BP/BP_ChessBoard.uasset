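; BP_ChessBoard is a chess board actor that spawns one BP_Pawn and one BP_ChessSquare at its own transform on BeginPlay.
; It first caches any existing BP_ChessSquare through GetActorOfClass and sets SquareCounter to one.
; After spawning, it stores the new square's CenterPivot world location in SquareArray.
; No grid loop exists, and neither the counter nor the cached reference drives the spawning.
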(event EventBeginPlay
  (CallFunction|SetChessSquareRef)
  (Variables|Setup|SetSquareCounter 1)
  (Game|SpawnActorfromClass "/Game/BP/BP_Pawn.BP_Pawn_C" (Transformation|GetActorTransform) "Undefined" 0 0)
  (bind _returnvalue (Game|SpawnActorfromClass "/Game/BP/BP_ChessSquare.BP_ChessSquare_C" (Transformation|GetActorTransform) "AlwaysSpawn" 0 0))
  (Utilities|Array|Add (Variables|Setup|GetSquareArray) (Transformation|GetWorldLocation (Variables|/Game/BP/BP_ChessSquare.BP_ChessSquare_C|GetCenterPivot _returnvalue))))

(fn ConstructionScript)

(fn SetChessSquareRef
  (Utilities|IsValid (Variables|Ref|GetChessSquareRef)
    (:Is%20Not%20Valid
      (bind _returnvalue (Actor|GetActorOfClass "/Game/BP/BP_ChessSquare.BP_ChessSquare_C"))
      (Variables|Ref|SetChessSquareRef _returnvalue))))