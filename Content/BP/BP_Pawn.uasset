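; BP_Pawn is a pawn set up to receive four-direction movement input from BP_PlayerController, with the movement itself not yet implemented.
; On BeginPlay it caches a cast reference to player controller 0 and binds to that controller's MoveFourDirections dispatcher.
; The bound event switches on Direction but has no branch logic, and MakeFourTransforms is an empty stub.
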(event Custom|MoveFourDirections
  (params (Direction :type Integer))
  (switch int Direction))

(event EventBeginPlay
  (Ref|SetPlayerControllerRef)
  (EventDispatchers|AssignMoveFourDirections (Variables|Ref|GetPlayerControllerRef) (EventDispatchers|CreateEvent :!event Custom|MoveFourDirections)))

(fn ConstructionScript)

(fn SetPlayerControllerRef
  (Utilities|IsValid (Variables|Ref|GetPlayerControllerRef)
    (:Is%20Not%20Valid
      (bind _asbp_player_controller (Utilities|Casting|CastToBP_PlayerController (Game|GetPlayerController 0)))
      (Variables|Ref|SetPlayerControllerRef _asbp_player_controller))))

(fn MakeFourTransforms)