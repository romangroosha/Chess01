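; Player controller that turns arrow key presses into four-direction move requests.
; On BeginPlay it caches typed references to itself and the BP_Pawn player pawn, then enables input.
; Each key press calls CallMoveFourDirections with a direction index; the movement logic is not defined in this graph.
; An unused GetActorOfClass pawn lookup is left disconnected in SetPawnRef.
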(event EventBeginPlay
  (Ref|SetPlayerControllerRef)
  (Ref|SetPawnRef)
  (Input|EnableInput (Game|GetPlayerController 0)))

(event Input|KeyboardEvents|Up
  (params (Key :type Key%20Structure :default "None"))
  (:Pressed
    (Default|CallMoveFourDirections)))

(event Input|KeyboardEvents|Left
  (params (Key :type Key%20Structure :default "None"))
  (:Pressed
    (Default|CallMoveFourDirections 3)))

(event Input|KeyboardEvents|Right
  (params (Key :type Key%20Structure :default "None"))
  (:Pressed
    (Default|CallMoveFourDirections 2)))

(event Input|KeyboardEvents|Down
  (params (Key :type Key%20Structure :default "None"))
  (:Pressed
    (Default|CallMoveFourDirections 1)))

(fn ConstructionScript)

(fn SetPlayerControllerRef
  (Utilities|IsValid (Variables|Default|GetPlayerControllerRef)
    (:Is%20Not%20Valid
      (bind _asbp_player_controller (Utilities|Casting|CastToBP_PlayerController (Game|GetPlayerController 0)))
      (Variables|Default|SetPlayerControllerRef _asbp_player_controller))))

(fn SetPawnRef
  (Utilities|IsValid (Variables|Default|GetPawnRef)
    (:Is%20Not%20Valid
      (bind _asbp_pawn (Utilities|Casting|CastToBP_Pawn (Game|Player|GetPlayerPawn 0)))
      (Variables|Default|SetPawnRef _asbp_pawn))))