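; BP_ChessSquare is a numbered board tile that grows a randomly shaped board by spawning the next tile, chaining until the BP_ChessBoard counter passes 255.
; On BeginPlay it shows the counter, then after a short delay spawns and registers a successor.
; Placement picks a random existing square, filters its four orthogonal neighbors against occupied locations, and retries if none remain.
; A timeline drives a dynamic material's color from violet to white.
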(event EventBeginPlay
  (bind _centerpivot (Variables|Default|GetCenterPivot))
  (bind _returnvalue (Transformation|GetWorldTransform _centerpivot))
  ;[1 1 1] Number on the Square
  (Ref|SetChessBoardRef)
  (Rendering|Components|TextRender|SetText (Variables|Default|GetTextRender) (Utilities|Text|ToText(Integer) (Variables|/Game/BP/BP_ChessBoard.BP_ChessBoard_C|GetSquareCounter (Variables|Ref|GetChessBoardRef))))
  (Utilities|FlowControl|Sequence
    (:then_0
      ;[1 1 1] How many squares
      (if (<= (Variables|/Game/BP/BP_ChessBoard.BP_ChessBoard_C|GetSquareCounter (Variables|Ref|GetChessBoardRef)) 255)
        (Variables|/Game/BP/BP_ChessBoard.BP_ChessBoard_C|SetSquareCounter (Variables|Ref|GetChessBoardRef) (+ (Variables|/Game/BP/BP_ChessBoard.BP_ChessBoard_C|GetSquareCounter (Variables|Ref|GetChessBoardRef)) 1))
        (Utilities|FlowControl|Delay 0.01)
        ;[1 1 1] Spawn New Square and Send it to SquareArray (in BP_ChessBoard)
        (bind _returnvalue_2 (Game|SpawnActorfromClass "BP_ChessSquare_C" (Math|Transform|MakeTransform (.Get%20Vector (Utility|GetRandomArrayIndex (Setup|CheckValidLocations (Variables|/Game/BP/BP_ChessBoard.BP_ChessBoard_C|GetSquareLocation (Variables|Ref|GetChessBoardRef)) (Variables|/Game/BP/BP_ChessBoard.BP_ChessBoard_C|GetSquareDistance (Variables|Ref|GetChessBoardRef))))) (.rotation _returnvalue) (.scale _returnvalue)) "Undefined" 0 0))
        (Utilities|Array|Add (Variables|/Game/BP/BP_ChessBoard.BP_ChessBoard_C|GetSquareLocation (Variables|Ref|GetChessBoardRef)) (Transformation|GetWorldLocation (Variables|BP_ChessSquare_C|GetCenterPivot _returnvalue_2)))
        (Utilities|Array|Add (Variables|/Game/BP/BP_ChessBoard.BP_ChessBoard_C|GetAll_Square (Variables|Ref|GetChessBoardRef)) 0)))
    (:then_1
      ;[1 1 1] Change Color over Time
      (bind _returnvalue_3 (Rendering|Material|CreateDynamicMaterialInstance (Variables|Default|GetCube) 0 "/Game/Materials/MT_ChessSquare.MT_ChessSquare" "None" :!class /Script/Engine.PrimitiveComponent))
      (bind _violet_to_white (Timeline|ChangeSquareColor_Timeline PlayFromStart)
        (:Update
          (Rendering|Material|SetVectorParameterValue _returnvalue_3 "Color" _violet_to_white :!class /Script/Engine.MaterialInstanceDynamic))))))

(fn ConstructionScript)

(fn SetChessBoardRef
  (Utilities|IsValid (Variables|Ref|GetChessBoardRef)
    (:Is%20Not%20Valid
      (bind _returnvalue (Actor|GetActorOfClass "/Game/BP/BP_ChessBoard.BP_ChessBoard_C"))
      (Variables|Ref|SetChessBoardRef _returnvalue))))

(fn FourLocations
  (params (Pivot%20Location :type Vector) (Distance :type Float%20%28double-precision%29))
  (LocalVariables|SetInputLoc Pivot%20Location)
  (LocalVariables|SetLocDistanceFloat Distance)
  (LocalVariables|SetLoc_1 (Math|Vector|MakeVector (+ (LocalVariables|GetLocDistanceFloat) (.x (LocalVariables|GetInputLoc))) (.y (LocalVariables|GetInputLoc)) (.z (LocalVariables|GetInputLoc))))
  (LocalVariables|SetLoc_2 (Math|Vector|MakeVector (+ (* (LocalVariables|GetLocDistanceFloat) -1.0) (.x (LocalVariables|GetInputLoc))) (.y (LocalVariables|GetInputLoc)) (.z (LocalVariables|GetInputLoc))))
  (LocalVariables|SetLoc_3 (Math|Vector|MakeVector (.x (LocalVariables|GetInputLoc)) (+ (LocalVariables|GetLocDistanceFloat) (.y (LocalVariables|GetInputLoc))) (.z (LocalVariables|GetInputLoc))))
  (LocalVariables|SetLoc_4 (Math|Vector|MakeVector (.x (LocalVariables|GetInputLoc)) (+ (* (LocalVariables|GetLocDistanceFloat) -1.0) (.y (LocalVariables|GetInputLoc))) (.z (LocalVariables|GetInputLoc))))
  (return (Utilities|Array|MakeArray (LocalVariables|GetLoc_1) (LocalVariables|GetLoc_2) (LocalVariables|GetLoc_3) (LocalVariables|GetLoc_4))))

(fn ClearAppendClear
  (params (Array%201 :type Array%20of%20Vectors) (Array%202 :type Array%20of%20Vectors))
  (Utilities|Array|Clear Array%201)
  (Utilities|Array|AppendArray Array%201 Array%202)
  (Utilities|Array|Clear Array%202))

(fn GetRandomArrayIndex
  (params (Array :type Array%20of%20Vectors))
  (bind _returnvalue (Utilities|Array|LastIndex Array))
  (bind _returnvalue_2 (Math|Random|RandomIntegerinRange 0 _returnvalue))
  (return (Utilities|Array|Get(acopy) Array _returnvalue_2) _returnvalue_2))

(fn CheckValidLocations
  (params (Square%20Array :type Array%20of%20Vectors) (Distance :type Float%20%28double-precision%29))
  (LocalVariables|SetLocal%20Square%20Array Square%20Array :!label _label)
  (LocalVariables|SetLocal%20Array%201 (Setup|FourLocations (.Get%20Vector (Utility|GetRandomArrayIndex Square%20Array)) Distance))
  (LocalVariables|SetLocal%20Array%202 (Utilities|Array|MakeArray))
  (bind _array_element (Utilities|Array|ForEachLoopwithBreak (LocalVariables|GetLocal%20Square%20Array))
    (:LoopBody
      (bind _array_element_2 (Utilities|Array|ForEachLoopwithBreak (LocalVariables|GetLocal%20Array%201))
        (:LoopBody
          (if (Utilities|Operators|NotEqual(!=) _array_element _array_element_2 0.0)
            (Utilities|Array|Add (LocalVariables|GetLocal%20Array%202) _array_element_2)))
        (:Completed
          (Utility|ClearAppendClear (LocalVariables|GetLocal%20Array%201) (LocalVariables|GetLocal%20Array%202)) ; On Completion, gives data \nfrom the second array \nto the first array
        )))
    (:Completed
      (if (Utilities|Array|IsEmpty (LocalVariables|GetLocal%20Array%201))
        (goto _label)
        (else
          (return (LocalVariables|GetLocal%20Array%201)))))))